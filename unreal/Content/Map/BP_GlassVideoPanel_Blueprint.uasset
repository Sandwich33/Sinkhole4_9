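; BP_GlassVideoPanel is a map actor that, going by its name, shows a video on a glass panel.
; BeginPlay starts the Video and Audio members together, playing the audio from time zero.
; Tick polls the video every frame and calls Pause on it whenever it is not playing.
; The overlap event is empty, and the construction script only calls its parent.
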(event `self.ReceiveBeginPlay`
  (`parent.ReceiveBeginPlay`)
  (`MediaPlayer.Play` (`self.video`))
  (`AudioComponent.Play` (`self.Audio`) 0.0))

(event `self.ReceiveActorBeginOverlap`
  (params (OtherActor :type "Actor Object Reference")))

(event `self.ReceiveTick`
  (params (DeltaSeconds :type "Float (single-precision)"))
  (`parent.ReceiveTick` 0.0)
  (if (not (`MediaPlayer.IsPlaying` (`self.video`)))
    (`MediaPlayer.Pause` (`self.video`))))

(fn `UserConstructionScript`
  (`parent.UserConstructionScript`))