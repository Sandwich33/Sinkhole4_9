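; Sinkhole HUD that draws the player's health bar and aiming crosshair on the canvas each frame.
; A dynamic material created at BeginPlay receives the Player_Person HP ratio and is drawn bottom-left beneath a frame texture.
; When GetAimInfo allows it, a textured crosshair draws at the aim point, falling back to screen center, with four outer markers that spread with recoil.
; An older red DrawLine crosshair remains unconnected.
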(event `self.ReceiveBeginPlay`
  (bind _returnvalue (`KismetMaterialLibrary.CreateDynamicMaterialInstance` "/Game/HUD/HpBar/M_hpBar.M_hpBar"))
  (set `self.hpBarInstance` _returnvalue))

(event `self.ReceiveDrawHUD`
  (params (SizeX :type Integer) (SizeY :type Integer))
  (bind _t_aimline (`self.T_aimLine`))
  (bind _t_aimline_2 (`self.T_aimLine`))
  (bind _t_r (`self.T_R`))
  (bind _t_r_2 (`self.T_R`))
  (bind (_x _y) (`KismetMathLibrary.BreakVector2D` (`self._draw_sp`)))
  (bind (_x_2 _y_2) (`KismetMathLibrary.BreakVector2D` (`self._draw_sp`)))
  (bind (_x_3 _y_3) (`KismetMathLibrary.BreakVector2D` (`self._draw_sp`)))
  (bind _returnvalue (* (`self.recoil`) 0.07))
  (bind _returnvalue_2 (* (`self.recoil`) 0.07))
  (bind _returnvalue_3 (- (`.Y` (`KismetMathLibrary.BreakVector2D` (`WidgetLayoutLibrary.GetViewportSize`))) 80.0))
  (`|ExecutionSequence`
    (:`then_0`
      ;[1 1 1] HP bar
      (bind _asplayer_person (cast `/Game/Blueprint/Characters/Player/Player_Person` (`GameplayStatics.GetPlayerPawn` 0)))
      (`MaterialInstanceDynamic.SetScalarParameterValue` (`self.hpBarInstance`) "healthPercentage" (/ (`/Game/Blueprint/Characters/Person_Character.hp` _asplayer_person) (`/Game/Blueprint/Characters/Person_Character.MAX_HP` _asplayer_person)))
      (`self.DrawMaterialSimple` (`self.hpBarInstance`) 20.0 _returnvalue_3 350.0 65.0)
      (`self.DrawTextureSimple` "/Game/HUD/HpBar/T_hpBarFrame.T_hpBarFrame" 20.0 _returnvalue_3 0.1))
    (:`then_1`
      (set `self._draw_sp` (`KismetMathLibrary.MakeVector2D` (`KismetMathLibrary.Conv_IntToDouble` (/ SizeX 2)) (`KismetMathLibrary.Conv_IntToDouble` (/ SizeY 2))))
      (bind _asplayer_person_2 (cast `/Game/Blueprint/Characters/Player/Player_Person` (`GameplayStatics.GetPlayerCharacter` 0)))
      (bind (__recoil __screen_point _showaim) (`/Game/Blueprint/Characters/Player/Player_Person.GetAimInfo` _asplayer_person_2))
      (if _showaim
        (set `self.recoil` __recoil)
        (bind (_x_4 _y_4) (`KismetMathLibrary.BreakVector2D` __screen_point))
        (if (not (<= (+ _x_4 _y_4) 0.0))
          (set `self._draw_sp` __screen_point))
        (`|ExecutionSequence`
          (:`then_0`
            (`self.DrawTexture` "/Game/HUD/crosshair_center.crosshair_center" (- _x 2.5) (- _y 2.5) 5.0 5.0 1.0 1.0 1.0 1.0 (struct :`R` 1.0 :`G` 1.0 :`B` 1.0 :`A` 1.0) "BLEND_Translucent" 1.0 false 0.0))
          (:`then_1`
            ;[1 1 1] Line
            (`|ExecutionSequence`
              (:`then_0`
                (`self.DrawTexture` _t_aimline (- _x_3 2.5) (- _y_3 33.0) 5.0 25.0 1.0 1.0 1.0 1.0 (struct :`R` 1.0 :`G` 1.0 :`B` 1.0 :`A` 1.0) "BLEND_Translucent" 1.0))
              (:`then_1`
                (`self.DrawTexture` _t_aimline (- _x_3 -2.5) (- _y_3 -33.0) 5.0 25.0 1.0 1.0 1.0 1.0 (struct :`R` 1.0 :`G` 1.0 :`B` 1.0 :`A` 1.0) "BLEND_Translucent" 1.0 false 180.0))
              (:`then_2`
                (`self.DrawTexture` _t_aimline_2 (- _x_3 -33.0) (- _y_3 2.5) 5.0 25.0 1.0 1.0 1.0 1.0 (struct :`R` 1.0 :`G` 1.0 :`B` 1.0 :`A` 1.0) "BLEND_Translucent" 1.0 false 90.0))
              (:`then_3`
                (`self.DrawTexture` _t_aimline_2 (- _x_3 33.0) (- _y_3 -2.5) 5.0 25.0 1.0 1.0 1.0 1.0 (struct :`R` 1.0 :`G` 1.0 :`B` 1.0 :`A` 1.0) "BLEND_Translucent" 1.0 false 270.0))))
          (:`then_2`
            ;[1 1 1] Line
            (`|ExecutionSequence`
              (:`then_0`
                (`self.DrawTexture` _t_r_2 (+ _x_2 _returnvalue_2) (- (- _y_2 _returnvalue_2) 10.0) 10.0 10.0 1.0 1.0 1.0 1.0 (struct :`R` 1.0 :`G` 1.0 :`B` 1.0 :`A` 1.0) "BLEND_Translucent" 1.0))
              (:`then_1`
                (`self.DrawTexture` _t_r_2 (- _x_2 _returnvalue_2) (+ (+ _y_2 _returnvalue_2) 10.0) 10.0 10.0 1.0 1.0 1.0 1.0 (struct :`R` 1.0 :`G` 1.0 :`B` 1.0 :`A` 1.0) "BLEND_Translucent" 1.0 false 180.0))
              (:`then_2`
                (`self.DrawTexture` _t_r (+ (+ _x_2 _returnvalue) 10.0) (+ _y_2 _returnvalue) 10.0 10.0 1.0 1.0 1.0 1.0 (struct :`R` 1.0 :`G` 1.0 :`B` 1.0 :`A` 1.0) "BLEND_Translucent" 1.0 false 90.0))
              (:`then_3`
                (`self.DrawTexture` _t_r (- (- _x_2 _returnvalue) 10.0) (- _y_2 _returnvalue) 10.0 10.0 1.0 1.0 1.0 1.0 (struct :`R` 1.0 :`G` 1.0 :`B` 1.0 :`A` 1.0) "BLEND_Translucent" 1.0 false 270.0)))))))))

(fn `UserConstructionScript`)