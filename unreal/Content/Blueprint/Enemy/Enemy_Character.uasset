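; Base enemy Character that takes damage, strikes non-enemy actors and alerts nearby enemies when attacked.
; Incoming damage from other enemies is ignored; the rest reduces Hp, with death disabling capsule collision and clearing AIControllerClass.
; Each hit sphere-traces for tagged enemies, which set the attacker as Blackboard TargetToAttack if untargeted or closer.
; CanAttack limits HitAttack to one hit; attack and sound functions are empty stubs, and HP bar creation is disconnected.
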(event EventBeginPlay)

(event EventTick
  (params (DeltaSeconds :type Float%20%28single-precision%29)))

(event Game|Damage|EventAnyDamage
  (params (Damage :type Float%20%28single-precision%29) (DamageType :type Damage%20Type%20Object%20Reference) (InstigatedBy :type Controller%20Object%20Reference) (DamageCauser :type Actor%20Object%20Reference))
  ;[1 1 1] Demage
  (Utilities|IsTeamKill false DamageCauser
    (:__
      (Utilities|FlowControl|Sequence
        (:then_0
          (Utilities|ApplyDemage Damage
            (:_die
              (CallFunction|OnDie))))
        (:then_1
          (CallFunction|AlarmGettingAttacked DamageCauser))))))

(fn ConstructionScript
  (Variables|Default|Sethp (Variables|Default|GetMAX_HP))
  (Variables|Default|SetTags (Utilities|Array|MakeArray "Enemy")))

(fn OnDie
  (bind _hp_bar (Variables|Default|Gethp_bar))
  (Variables|Default|SetAIControllerClass 0)
  (Collision|SetCollisionEnabled (Variables|Collision|GetCapsuleComponent) "NoCollision")
  (Utilities|IsValid _hp_bar
    (:Is%20Valid
      (Widget|RemovefromParent _hp_bar))))

(fn SetCanAttack
  (params (_can_attack :type Boolean))
  (bind _output_get (Variables|Default|Setcan_attack _can_attack))
  (if _output_get
    _
    (else
      _))
  (return))

(fn HitAttack
  (params (_hit :type Hit%20Result%20Structure) (_other_actor :type Actor%20Object%20Reference))
  (if (Variables|Default|Getcan_attack)
    (Utilities|Casting|CastToEnemy_Character _other_actor
      (:CastFailed
        (Game|Damage|ApplyDamage (.HitActor (Collision|BreakHitResult _hit)) (Variables|Default|GetDAMAGE) 0 self)
        (CallFunction|SetCanAttack false)))))

(fn OnAttack)

(fn AlarmGettingAttacked
  (params (_damageCauser :type Actor%20Object%20Reference))
  (bind _self self)
  (bind _returnvalue (Transformation|GetActorLocation _self))
  (bind _outhits (Collision|MultiSphereTraceForObjects _returnvalue (+ _returnvalue "0, 0,10.000000") 2e+03 (Utilities|Array|MakeArray "ObjectTypeQuery3") false 0 "None" false))
  (for _array_element _outhits
    (if (Utilities|Name|Equal(Name) (Utilities|Array|Get(acopy) (Variables|/Script/Engine.Actor|GetTags (.HitActor (Collision|BreakHitResult _array_element)))) "Enemy")
      (bind _asenemy_character (Utilities|Casting|CastToEnemy_Character (.HitActor (Collision|BreakHitResult _array_element))))
      (CallFunction|ReceiveAttackAlarm _asenemy_character _damageCauser))))

(fn ReceiveAttackAlarm
  (params (_damageCauser :type Actor%20Object%20Reference))
  (bind _self self)
  (bind _self_2 self)
  (bind _targettoattack (LocalVariables|GettargetToAttack))
  (bind _returnvalue (Transformation|GetActorLocation _self_2))
  (bind _returnvalue_2 (AI|GetBlackboard _self))
  (bind _returnvalue_3 (AI|Components|Blackboard|GetValueasObject _returnvalue_2 _targettoattack))
  ;[1 1 1] 타겟이 없으면 공격자를 타겟으로 설정
  (if (== _returnvalue_3 0)
    (AI|Components|Blackboard|SetValueasObject (AI|GetBlackboard self) (LocalVariables|GettargetToAttack) _damageCauser :!label _label)
    (else
      ;[1 1 1] 타겟이 있으면, 공격자가 타겟보다 가까울 때 타겟으로 설정
      (bind _asactor (Utilities|Casting|CastToActor _returnvalue_3))
      (if (< (Math|Vector|VectorLength (- (Transformation|GetActorLocation _damageCauser) _returnvalue)) (Math|Vector|VectorLength (- (Transformation|GetActorLocation _asactor) _returnvalue)))
        (goto _label)))))

(fn PlayAttackSound)

(fn PlayDieSound)

(fn PlayAttackSound2)

(fn PlayAttackSound3)