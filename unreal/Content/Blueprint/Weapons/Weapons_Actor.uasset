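; Base-style weapon actor that handles hitscan firing, ammo, reloading and recoil spread, with empty hooks for sounds, particles and reload animation.
; Aim traces run from the gun's AimSocket along a camera actor's forward vector and also yield a screen point.
; Each shot trace widens a capped recoil range that randomizes the endpoint and decays while waiting.
; A delta-time countdown paces fire, while DoFire applies point damage and spends a bullet.
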(fn ConstructionScript
  (Class|SceneComponent|Attachto (Variables|Default|GetCamera) (Variables|Default|GetGunMesh) "ZoomSocket" "KeepRelativeOffset" true))

(fn ActionFire
  (params (_pressed :type Boolean))
  (bind _output_get (Variables|Fire|Setcan_fire _pressed))
  (if _output_get
    (return true)
    (else
      (return false))))

(fn DoFire
  (params (_demabe_causer :type Actor%20Object%20Reference) (_hit_info :type Hit%20Result%20Structure))
  (bind (_bblockinghit _binitialoverlap _time _location _impactpoint _normal _impactnormal _physmat _hitactor) (Collision|BreakHitResult _hit_info))
  (Game|Damage|ApplyPointDamage _hitactor (Variables|Default|GetDEMAGE) _impactnormal _hit_info 0 _demabe_causer)
  (Math|Integer|DecrementInt (Variables|Default|Getin_bullet)))

(fn GetAim
  (bind _gunmesh (Variables|Default|GetGunMesh))
  (bind _returnvalue (Transformation|GetSocketLocation _gunmesh "AimSocket"))
  (bind __return_value (CallFunction|GetLookVector))
  (bind _output_get (LocalVariables|Setstart_location _returnvalue))
  (bind _output_get_2 (LocalVariables|Setend_location (+ _returnvalue (* __return_value (Variables|Fire|GetRANGE)))))
  (bind (_outhit _returnvalue_2) (Collision|LineTraceByChannel _output_get _output_get_2 "TraceTypeQuery1" false 0 "None"))
  (if _returnvalue_2
    (bind _asplayer_controller (Utilities|Casting|CastToPlayerController (Variables|Default|Getplayer_controller))
      (:then
        (LocalVariables|Setscreen_point (.ScreenLocation (Class|PlayerController|ProjectWorldLocationtoScreen _asplayer_controller (.Location (Collision|BreakHitResult _outhit))))))
      (:CastFailed
        (LocalVariables|Setscreen_point "" :!label _label)))
    (else
      (goto _label)))
  (return (LocalVariables|Getstart_location) (LocalVariables|Getend_location) (LocalVariables|Getscreen_point)))

(fn DelayFire
  (params (_delta_seconds :type Float%20%28single-precision%29))
  (bind _output_get (Variables|Fire|Setdelta_time (- (Variables|Fire|Getdelta_time) _delta_seconds)))
  (if (<= _output_get 0.0)
    (Variables|Fire|Setdelta_time (Variables|Fire|GetFIRE_SPEED))
    (return true)
    (else
      (return false))))

(fn OnFire?
  (if (<= (Variables|Default|Getin_bullet) 0)
    (Variables|Fire|Setcan_fire false))
  (return (Variables|Fire|Getcan_fire)))

(fn CreateParticle)

(fn PlayFireSound)

(fn GetDemageActor
  (params (_in_aim_data :type Boolean) (_start_location :type Vector) (_end_location :type Vector))
  (bind _recoil (Variables|Fire|Getrecoil))
  (bind _returnvalue (* _recoil -1.0))
  (bind (__out_start_location __out_end_location __object_type) (CallFunction|GetRecoilLine _in_aim_data _start_location _end_location))
  (bind (_outhit _returnvalue_2) (Collision|LineTraceForObjects __out_start_location (+ __out_end_location (Math|Vector|MakeVector (Math|Random|RandomFloatinRange _returnvalue _recoil) (Math|Random|RandomFloatinRange _returnvalue _recoil) (Math|Random|RandomFloatinRange _returnvalue _recoil))) __object_type false 0 "None"))
  (if _returnvalue_2
    (Effects|SpawnEmitteratLocation "/Game/Effects/Impacts/P_Impact_Metal_Blossom.P_Impact_Metal_Blossom" (.Location (Collision|BreakHitResult _outhit))))
  (return (Utilities|Array|MakeArray _outhit) _returnvalue_2))

(fn ActionReload
  (params (_total_bullet :type Integer))
  (bind _max_bullet (Variables|Default|GetMAX_BULLET))
  (LocalVariables|Settemp (- _total_bullet (- _max_bullet (Variables|Default|Getin_bullet))))
  (if (> (- _total_bullet (- _max_bullet (Variables|Default|Getin_bullet))) 0)
    (Variables|Default|Setin_bullet (Variables|Default|GetMAX_BULLET))
    (return (LocalVariables|Gettemp))
    (else
      (Variables|Default|Setin_bullet (+ _max_bullet (- _total_bullet (- _max_bullet (Variables|Default|Getin_bullet)))))
      (return 0))))

(fn OnReloadAnimation)

(fn WaitingFire
  (params (_delta_seconds :type Float%20%28single-precision%29))
  (bind _recoil_default (Variables|Fire|GetRECOIL_DEFAULT))
  (if (> (Variables|Fire|Getdelta_time) 0.0)
    (Variables|Fire|Setdelta_time (- (Variables|Fire|Getdelta_time) _delta_seconds)))
  ;[1 1 1] 연사와 반동
  (if (< (- (Variables|Fire|Getrecoil_range) (/ (Variables|Fire|GetRECOIL_RANGE_MAX) 2e+01)) 0.0)
    (Variables|Fire|Setrecoil_range 0.0)
    (Variables|Fire|Setrecoil _recoil_default)
    (else
      (bind _output_get (Variables|Fire|Setrecoil_range (- (Variables|Fire|Getrecoil_range) (/ (Variables|Fire|GetRECOIL_RANGE_MAX) 2e+01))))
      (Variables|Fire|Setrecoil (+ _output_get _recoil_default)))))

(fn GetRecoilLine
  (params (_in_aim_data :type Boolean) (_start_location :type Vector) (_end_location :type Vector))
  (bind _array (Utilities|Array|MakeArray "ObjectTypeQuery3" "ObjectTypeQuery6" "ObjectTypeQuery1"))
  (bind _recoil_default (Variables|Fire|GetRECOIL_DEFAULT))
  (bind _recoil_range_max (Variables|Fire|GetRECOIL_RANGE_MAX))
  (Utilities|FlowControl|Sequence
    (:then_0
      ;[1 1 1] 연사와 반동
      (if (< (+ (Variables|Fire|Getrecoil_range) (/ _recoil_range_max 2e+01)) _recoil_range_max)
        (bind _output_get (Variables|Fire|Setrecoil_range (+ (Variables|Fire|Getrecoil_range) (/ _recoil_range_max 2e+01))))
        (Variables|Fire|Setrecoil (+ _output_get _recoil_default))
        (else
          (bind _output_get_2 (Variables|Fire|Setrecoil_range _recoil_range_max))
          (Variables|Fire|Setrecoil (+ _output_get_2 _recoil_default)))))
    (:then_1
      (if _in_aim_data
        (return _start_location _end_location _array)
        (else
          (bind (__start_location __end_location) (CallFunction|GetAim))
          (return __start_location __end_location _array))))))

(fn GetLookVector
  (return (Math|Vector|GetForwardVector (Variables|Default|Getcamera_actor))))

(fn PlayReloadSound)

(fn PlayZoominSound)

(fn GetAimInfo
  (return (Variables|Fire|Getrecoil)))