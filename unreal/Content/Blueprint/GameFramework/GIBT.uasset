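; GIBT is a game-framework Blueprint that manages a local TCP client connection labelled connectTablet and keeps it through level changes.
; TryConnect uses a Not/Checking/Connect state to create the localhost socket once, then reports whether it is connected.
; OpenLV sets ReasonLevel before loading a level, so CloseLV skips teardown until Init clears the flag.
; Otherwise, DestoryNet sends a MainActivity action message and destroys the connected client.
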(fn `closeLV`
  (if (not (`self.reason_level`))
    (`self.destoryNet`)))

(fn `destoryNet`
  (switch `/Game/Tablet/NetConnectState` (`self.net_connect_state`)
    (:`NewEnumerator2`
      (if (not (`self.reason_level`))
        (`OneNetworking.sendMessage` (`self.one_network`) "act;MainActivity")
        (`OneNetworking.Destructor` (`self.one_network`))))))

(fn `init`
  (set `self.reason_level` false))

(fn `openLV`
  (params (_level_name :type Name))
  (set `self.reason_level` true)
  (`GameplayStatics.OpenLevel` _level_name))

(fn `tryConnect`
  (returns (_is_connect :type Boolean))
  (switch `/Game/Tablet/NetConnectState` (`self.net_connect_state`)
    (:`NewEnumerator0`
      ;[1 1 1] Try Connect
      (set `self.net_connect_state` "NewEnumerator1")
      (bind _output_get (set `self.one_network` (`OneNetworking.createTCPClient` "connectTablet" "127.0.0.1" 27015)))
      (bind _returnvalue (`OneNetworking.isConnection` _output_get))
      (if _returnvalue
        (set `self.net_connect_state` "NewEnumerator2")
        (return true)
        (else
          (set `self.net_connect_state` "NewEnumerator0")
          (return false))))
    (:`NewEnumerator1`
      (return false))
    (:`NewEnumerator2`
      (bind _returnvalue_2 (`OneNetworking.isConnection` (`self.one_network`)))
      (if _returnvalue_2
        (return true)
        (else
          (return false))))))