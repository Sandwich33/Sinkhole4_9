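; Gear train actor that spins two medium and two small gears with a looping gear sound.
; Tick eases a shared rotation rate toward full or zero based on Active, set true at BeginPlay, then applies per-gear ratios and alternating directions.
; BeginPlay spawns the loop on MedGear2 as COGAudio, while Tick scales DoorAudio volume and pitch with rotation rate.
; GrabInteract is a stub returning zero.
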(event `self.ReceiveBeginPlay`
  (set `self.Active` true)
  (`/Engine/EditorBlueprintResources/StandardMacros.DoOnce` false :!label _label
    (:`Completed`
      (bind _returnvalue (`GameplayStatics.SpawnSoundAttached` "/Game/Assets/Audio/Communication_Gears_Loop_Cue.Communication_Gears_Loop_Cue" (`self.Med gear 2`) "None" (0.0 0.0 0.0) (struct) "EAttachLocation::KeepRelativeOffset" false 1.0 1.0))
      (set `self.COG Audio ` _returnvalue))))

(event `self.COG Audio .OnAudioFinished`
  (goto _label :!via `Reset`))

(event `self.ReceiveTick`
  (params (DeltaSeconds :type "Float (single-precision)"))
  (bind _door_audio (`self.Door Audio`))
  (bind _returnvalue (* (`self.Rotation rate`) DeltaSeconds))
  (bind _returnvalue_2 (`KismetMathLibrary.FClamp` (`KismetMathLibrary.MapRangeUnclamped` (`self.Rotation rate`) 0.0 10.0 0.0 1.0)))
  (set `self.Rotation rate` (`KismetMathLibrary.FInterpTo` (`self.Rotation rate`) (`KismetMathLibrary.SelectFloat` 40.0 0.0 (`self.Active`)) DeltaSeconds 5.0)) ; Rotation rate value blends to full speed smoothly
  (`SceneComponent.K2_AddLocalRotation` (`self.Med gear 1`) (`KismetMathLibrary.MakeRotator` 0.0 0.0 (* _returnvalue -1.0)) false false)
  (`SceneComponent.K2_AddLocalRotation` (`self.Med gear 2`) (`KismetMathLibrary.MakeRotator` 0.0 0.0 _returnvalue) false false)
  (`SceneComponent.K2_AddLocalRotation` (`self.Little gear 1`) (`KismetMathLibrary.MakeRotator` 0.0 0.0 (* _returnvalue 2.667)) false false)
  (`SceneComponent.K2_AddLocalRotation` (`self.Little gear 2`) (`KismetMathLibrary.MakeRotator` 0.0 0.0 (* _returnvalue -7.11)) false false)
  (`AudioComponent.SetVolumeMultiplier` _door_audio _returnvalue_2)
  (`AudioComponent.SetPitchMultiplier` _door_audio _returnvalue_2))

(fn `Grab interact`
  (params (`Player aim movement` :type "Vector2D Structure") (Interacting :type Boolean))
  (returns (`Player focus target` :type "Vector Structure"))
  (return (0.0 0.0 0.0)))

(fn `UserConstructionScript`)